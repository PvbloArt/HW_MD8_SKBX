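; BP_Bonus is a bonus actor that travels through the level until it hits a kill Z volume.
; Tick moves it with a swept world offset scaled by Speed, Direction and delta time.
; Overlapping a KillZVolume fires OnDead, destroys the actor and spawns an enlarged sparks emitter at the volume's root location rather than its own.
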(event EventBeginPlay)

(event Collision|EventActorBeginOverlap
  (params (OtherActor :type Actor%20Object%20Reference))
  (Utilities|Casting|CastToKillZVolume OtherActor)
  (Default|CallOnDead)
  (Actor|DestroyActor)
  (Effects|SpawnEmitteratLocation "/Game/StarterContent/Particles/P_Sparks.P_Sparks" (Transformation|GetWorldLocation (Variables|/Script/Engine.Actor|GetRootComponent OtherActor)) "0, 0, 0" "3.000000,3.000000,3.000000"))

(event EventTick
  (params (DeltaSeconds :type Float%20%28single-precision%29))
  (Transformation|AddActorWorldOffset (* DeltaSeconds (* (Variables|Default|GetSpeed) (Variables|Default|GetDirection))) true))

(fn ConstructionScript)