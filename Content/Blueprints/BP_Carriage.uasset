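; BP_Carriage is a player-controlled paddle that launches balls and collects bonus pickups.
; MoveRight input shifts it sideways in fixed, swept steps each frame, independent of delta time.
; SpawnBall runs at BeginPlay, spawning a ball at SpawnerBall, binding its OnDead event, decrementing Life and printing it when low.
; Hitting a BP_Bonus destroys it and spawns an extra ball, which has no OnDead binding or Life cost.
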(event EventBeginPlay
  (CallFunction|SpawnBall))

(event EventTick
  (params (DeltaSeconds :type Float%20%28single-precision%29)))

(event Collision|EventHit
  (params (MyComp :type Primitive%20Component%20Object%20Reference) (Other :type Actor%20Object%20Reference) (OtherComp :type Primitive%20Component%20Object%20Reference) (bSelfMoved :type Boolean) (HitLocation :type Vector :default "0, 0, 0") (HitNormal :type Vector :default "0, 0, 0") (NormalImpulse :type Vector :default "0, 0, 0") (Hit :type Hit%20Result%20Structure%20%28by%20ref%29))
  (bind _asbp_bonus (Utilities|Casting|CastToBP_Bonus Other))
  (Variables|Default|SetBonus _asbp_bonus)
  (CallFunction|BonusBall)
  (if true
    (Actor|DestroyActor Other)))

(event Input|AxisEvents|InputAxisMoveRight
  (params (AxisValue :type Float%20%28single-precision%29))
  (if (< AxisValue 0.0)
    (Transformation|AddActorWorldOffset "0,-50.000000, 0" true)))

(event Input|AxisEvents|InputAxisMoveRight
  (params (AxisValue :type Float%20%28single-precision%29))
  (if (> AxisValue 0.0)
    (Transformation|AddActorWorldOffset "0,50.000000, 0" true)))

(fn ConstructionScript)

(fn SpawnBall
  (bind _returnvalue (Game|SpawnActorfromClass "/Game/Blueprints/BP_Ball.BP_Ball_C" (Transformation|GetWorldTransform (Variables|Default|Getspawner_ball)) "AlwaysSpawn" "MultiplyWithRoot" 0 0))
  (bind _output_get (Variables|Default|SetPlayingBall _returnvalue))
  (EventDispatchers|BindEventtoOnDead _output_get (EventDispatchers|CreateEvent :!event SpawnBall))
  (bind _result (Math|Integer|DecrementInt (Variables|Default|Getlife))
    (:%20%20
      (bind _output_get_2 (Variables|Default|Setlife _result))
      (if (<= _output_get_2 1)
        (Development|PrintString (Utilities|String|ToString(Integer) (Variables|Default|Getlife)))
        (return)))))

(fn BonusBall
  (Game|SpawnActorfromClass "/Game/Blueprints/BP_Ball.BP_Ball_C" (Transformation|GetWorldTransform (Variables|Default|Getspawner_ball)) "AlwaysSpawn" "MultiplyWithRoot" 0 0))